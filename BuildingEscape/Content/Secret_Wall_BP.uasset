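; Secret wall actor that swings open around yaw and closes on calls through the OpenSecretWall interface.
; Opening plays the WallOpen timeline, adding yaw to the starting rotation with a timed creak sound.
; Closing snaps rotation to zero and rewinds the timeline, while Tick stops the creak and uses a DoOnce for one door slam.
; The animated WallClose timeline logic is disconnected and never runs.
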(event `self.ReceiveBeginPlay`
  (set `self.Initial Rotation` (`self.K2_GetActorRotation`)))

(event `self.OpenSecretWall.OnOpen`
  (set `self.firstOpen` true)
  (set `self.isOpen` true)
  (bind (_direction _wallopen) (`Timeline|WallOpen` :!label _label)
    (:`Update`
      (`self.K2_SetActorRotation` (`KismetMathLibrary.ComposeRotators` (`KismetMathLibrary.MakeRotator` 0.0 0.0 _wallopen) (`self.Initial Rotation`))))
    (:`Sound Timing`
      (bind _returnvalue (`GameplayStatics.SpawnSoundAtLocation` "/Game/Audio/137143__d-w__creaking-wooden-door-0002.137143__d-w__creaking-wooden-door-0002" (`self.K2_GetActorLocation`) (struct) 1.0 1.0 0.1 null null (stale `self.OpenSecretWall.OnClose` _output_get))))))

(event `self.OpenSecretWall.OnClose`
  (`self.K2_SetActorRotation` (struct))
  (bind _output_get (set `self.isOpen` false))
  (set `self.ResetTime` 0.0)
  (goto _label :!via `SetNewTime`))

(event `self.ReceiveTick`
  (params (DeltaSeconds :type "Float (single-precision)"))
  (if (`self.firstOpen`)
    (if (`self.isOpen`)
      (goto _label_2 :!via `Reset`)
      (else
        (`AudioComponent.Stop` (stale `self.OpenSecretWall.OnOpen` _returnvalue))
        (`/Engine/EditorBlueprintResources/StandardMacros.DoOnce` false :!label _label_2
          (:`Completed`
            (`GameplayStatics.SpawnSoundAtLocation` "/Game/Audio/155523__planet-leader__doorslam2.155523__planet-leader__doorslam2" (`self.K2_GetActorLocation`))))))))

(fn `UserConstructionScript`)